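; AI controller for patrolling guard NPCs that runs the PatrollingGuardBehavior tree on the PatrolData blackboard.
; BeginPlay seeds the blackboard's enemy key with the player pawn before starting the tree.
; AI perception updates set that key to sensed actors lacking the "Enemy" tag and clear it when sensing fails.
; FindPatrolRoute, which writes the guard's first patrol point as a waypoint, is deprecated in favour of the tree.
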(event `self.ReceiveBeginPlay`
  (bind _blackboardcomponent (`self.UseBlackboard` "/Game/Dynamic/NPC/AI/PatrolData.PatrolData"))
  (bind _output_get (set `self.BlackboardComp` _blackboardcomponent))
  (`BlackboardComponent.SetValueAsObject` _output_get (`self.Enemy Key`) (`GameplayStatics.GetPlayerPawn` 0))
  (`self.RunBehaviorTree` "/Game/Dynamic/NPC/AI/PatrollingGuardBehavior.PatrollingGuardBehavior"))

(event `self.ReceiveTick`
  (params (DeltaSeconds :type "Float (single-precision)")))

(event `self.AIPerception.OnTargetPerceptionUpdated`
  (params (Actor :type "Actor Object Reference") (Stimulus :type "AIStimulus Structure"))
  (bind _enemy_key (`self.Enemy Key`))
  (bind _blackboardcomp (`self.BlackboardComp`))
  (if (`self.ActorHasTag` Actor "Enemy")
    _
    (elif (`.bSuccessfullySensed` (break `AIStimulus` Stimulus))
      (`BlackboardComponent.SetValueAsObject` _blackboardcomp _enemy_key Actor)
      (else
        (`BlackboardComponent.ClearValue` _blackboardcomp _enemy_key)))))

(fn `Find Patrol Route`
  (params (`Blackboard Input` :type "BlackboardComponent Object Reference"))
  (bind _aspatrolling_guard_bp (cast `/Game/ThirdPersonCPP/Blueprints/PatrollingGuard_BP` (`self.K2_GetPawn`)))
  (`BlackboardComponent.SetValueAsObject` `Blackboard Input` "Waypoint" (`|GetArrayItem` (`/Game/ThirdPersonCPP/Blueprints/PatrollingGuard_BP.Patrol Points` _aspatrolling_guard_bp))))

(fn `UserConstructionScript`)